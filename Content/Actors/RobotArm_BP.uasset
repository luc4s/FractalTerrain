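; RobotArm_BP is a robot arm actor built on a poseable mesh, exposing its bones for other code to use.
; The construction script resolves each entry in BoneNames to a mesh bone index, and GetBones returns those indices with the BoneAxes array.
; BeginPlay clears the setting-up state, while SetupArm is a stub that only casts the player to MyCharacter.
; No logic here moves the arm, and its Timeline is unwired.
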(event `self.ReceiveBeginPlay`
  (`self.SetSettingUp` false))

(event `self.ReceiveTick`
  (params (DeltaSeconds :type "Float (single-precision)")))

(fn `GetBones`
  (returns (indices :type "Array of Integer") (axes :type "Array of Axe Enum"))
  (return (`self.BoneIndices`) (`self.BoneAxes`)))

(fn `SetupArm`
  (cast `MyCharacter` (`GameplayStatics.GetPlayerCharacter` 0)))

(fn `UserConstructionScript`
  (for (_array_element _array_index) (`self.BoneNames`)
    (`KismetArrayLibrary.Array_Set` (`self.BoneIndices`) _array_index (`SkinnedMeshComponent.GetBoneIndex` (`self.PoseableMesh`) _array_element) true)))