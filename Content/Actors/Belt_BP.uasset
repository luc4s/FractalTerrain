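; Conveyor belt actor that carries one item at a time and hands it to the belt in front.
; After a short BeginPlay delay, it picks its straight, corner or junction mesh from a bitmask of Back/Left/Right overlaps tagged BeltFront, then refreshes the front neighbor's mesh.
; While full, Tick plays a timeline lerping the item to the ItemEnd socket, clearing the slot once the next belt accepts it.
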(event `self.ReceiveBeginPlay`
  (bind _overlappingactors (`PrimitiveComponent.GetOverlappingActors` (`self.Front`) null))
  (`KismetSystemLibrary.Delay` 0.2)
  (`self.UpdateMesh`)
  (`/Engine/EditorBlueprintResources/StandardMacros.CompareInt` (`KismetArrayLibrary.Array_Length` _overlappingactors)
    (:`>`
      (bind _asbelt_bp (cast `/Game/Actors/Belt_BP` (`|GetArrayItem` _overlappingactors)))
      (`self.UpdateMesh` _asbelt_bp))))

(event `self.ReceiveTick`
  (params (DeltaSeconds :type "Float (single-precision)"))
  (bind _overlappingactors (`PrimitiveComponent.GetOverlappingActors` (`self.Front`) "Belt_BP_C"))
  (if (`self.Full`)
    (bind (_direction _value) (`Timeline|Timeline_0`)
      (:`Update`
        (`self.K2_SetActorLocation` (`self.Item`) (`KismetMathLibrary.VLerp` (.location (`self.ItemStartTrans`)) (.location (`SceneComponent.GetSocketTransform` (`self.StaticMesh`) "ItemEnd" "RTS_World")) _value) false false))
      (:`Finished`
        (if (`KismetArrayLibrary.Array_IsValidIndex` _overlappingactors)
          (bind _asbelt_bp (cast `/Game/Actors/Belt_BP` (`|GetArrayItem` _overlappingactors)))
          (bind _itemtaken (`self.AddItem` _asbelt_bp (`self.Item`)))
          (if _itemtaken
            (set `self.Full` false)
            (set `self.Item` null)
            (`TimelineComponent.SetPlaybackPosition` (`self.Timeline_0`) 0.0 false false)))))))

(fn `AddItem`
  (params (NewParam :type "Actor Object Reference"))
  (returns (ItemTaken :type Boolean))
  (if (`self.Full`)
    (return false)
    (else
      (bind _output_get (set `self.Item` NewParam))
      (set `self.Full` true)
      (set `self.ItemStartTrans` (`self.GetTransform` _output_get))
      (return true))))

(fn `ConnectsToBelt`
  (params (NewParam :type "BoxComponent Object Reference (by ref)"))
  (returns (Collides :type Boolean))
  (for _array_element (`PrimitiveComponent.GetOverlappingComponents` NewParam)
    (for _array_element_2 (`ActorComponent.ComponentTags` _array_element)
      (if (== _array_element_2 "BeltFront")
        (return true))))
  (return false))

(fn `GetBeltMesh`
  (params (NewParam :type "Integer (by ref)"))
  (returns (StaticMesh :type "StaticMesh Object Reference"))
  (switch `int` NewParam
    (:`0`
      _)
    (:`1`
      _)
    (:`2`
      (return "/Game/Assets/Belt/belt_left.belt_left"))
    (:`3`
      (return "/Game/Assets/Belt/belt_fwd_left.belt_fwd_left"))
    (:`4`
      (return "/Game/Assets/Belt/belt_right.belt_right"))
    (:`5`
      (return "/Game/Assets/Belt/belt_fwd_right.belt_fwd_right"))
    (:`6`
      (return "/Game/Assets/Belt/belt_all.belt_all"))
    (:`7`
      (return "/Game/Assets/Belt/belt_all.belt_all")))
  (return "/Game/Assets/Belt/belt_straight.belt_straight"))

(fn `GetCenterTransform`
  (returns (NewParam :type "Transform Structure"))
  (return (`SceneComponent.GetSocketTransform` (`self.StaticMesh`) "Center" "RTS_World")))

(fn `UpdateMesh`
  (locals (Sides :type Integer :default 0))
  (set `local.Sides` 0)
  (bind _collides (`self.ConnectsToBelt` (`self.Back`)))
  (if _collides
    (set `local.Sides` 1))
  (bind _collides_2 (`self.ConnectsToBelt` (`self.Left`)))
  (if _collides_2
    (set `local.Sides` (`KismetMathLibrary.Or_IntInt` (`local.Sides`) 2)))
  (bind _collides_3 (`self.ConnectsToBelt` (`self.Right`)))
  (if _collides_3
    (set `local.Sides` (`KismetMathLibrary.Or_IntInt` (`local.Sides`) 4)))
  (bind _staticmesh (`self.GetBeltMesh` (`local.Sides`)))
  (`StaticMeshComponent.SetStaticMesh` (`self.StaticMesh`) _staticmesh))

(fn `UserConstructionScript`)